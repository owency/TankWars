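; Player-controllable tank Blueprint that wires up its components and handles aim and fire input.
; On BeginPlay it passes the Barrel and TankTurret components to SetBarrelAndTurretReference.
; Aim axes orbit the view with frame-rate-scaled rotation, split gimbal-style: yaw on the Scene component, pitch on the SpringArm.
; The Fire action calls Fire, which, like the reference setter, is defined outside these graphs.
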(event EventBeginPlay
  (Class|Tank|SetBarrelandTurretReference (Variables|Default|GetBarrel) (Variables|Default|GetTankTurret)))

(event Input|ActionEvents|InputActionFire
  (params (Key :type Key%20Structure))
  (:Pressed
    (Class|Tank|Fire)))

(event Input|AxisEvents|InputAxisAimAzimuth
  (params (AxisValue :type Float%20%28single-precision%29))
  (Transformation|AddLocalRotation (Variables|Default|GetScene) (Math|Rotator|MakeRotator 0.0 0.0 (* AxisValue (Utilities|Time|GetWorldDeltaSeconds) 1e+02)) false false))

(event Input|AxisEvents|InputAxisAimAltitude
  (params (AxisValue :type Float%20%28single-precision%29))
  (Transformation|AddLocalRotation (Variables|Default|GetSpringArm) (Math|Rotator|MakeRotator 0.0 (* AxisValue (Utilities|Time|GetWorldDeltaSeconds) 1e+02) 0.0) false false))

(fn ConstructionScript)